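; BP_PMWall is a wall actor with a GeneratedWall procedural mesh component that responds to cursor hover, clicks and overlaps.
; On BeginPlay it caches the CB_PlayerController; hovering applies a preview material when that controller's wall mode is off, and leaving restores drywall.
; Clicks, overlaps and the hovered mesh's section count only print debug strings.
; The construction script is empty, so no geometry is built in this Blueprint.
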(event OnClicked(GeneratedWall)
  (params (TouchedComponent :type Primitive%20Component%20Object%20Reference) (ButtonPressed :type Key%20Structure :default "None"))
  (Development|PrintString "CLICKED!!"))

(event OnBeginCursorOver(GeneratedWall)
  (params (TouchedComponent :type Primitive%20Component%20Object%20Reference))
  (bind _generatedwall (Variables|Default|GetGeneratedWall))
  (bind _player_controller_ref (Variables|Default|GetPlayer%20Controller%20Ref))
  (Utilities|IsValid _player_controller_ref
    (:Is%20Valid
      (if (not (Variables|/Game/Character/CB_PlayerController.CB_PlayerController_C|GetWallModeEnabled _player_controller_ref))
        (Rendering|Material|SetMaterial _generatedwall 0 "/Game/Materials/M_WallPreview.M_WallPreview")
        (Development|PrintString (Utilities|String|ToString(Integer) (Class|ProceduralMeshComponent|GetNumSections _generatedwall)))))))

(event OnEndCursorOver(GeneratedWall)
  (params (TouchedComponent :type Primitive%20Component%20Object%20Reference))
  (Rendering|Material|SetMaterial (Variables|Default|GetGeneratedWall) 0 "/Game/Megascans/Surfaces/Drywall/Drywall_uhrmcixn_inst.Drywall_uhrmcixn_inst"))

(event OnComponentBeginOverlap(GeneratedWall)
  (params (OverlappedComponent :type Primitive%20Component%20Object%20Reference) (OtherActor :type Actor%20Object%20Reference) (OtherComp :type Primitive%20Component%20Object%20Reference) (OtherBodyIndex :type Integer) (bFromSweep :type Boolean) (SweepResult :type Hit%20Result%20Structure%20%28by%20ref%29))
  (Development|PrintString "Overlapping")
  (Development|PrintString (Utilities|GetObjectName OtherActor)))

(event EventBeginPlay
  (bind _outactors (Actor|GetAllActorsOfClass "/Game/Character/CB_PlayerController.CB_PlayerController_C"))
  (Variables|Default|SetPlayer%20Controller%20Ref (Utilities|Array|Get(acopy) _outactors)))

(event Collision|EventActorBeginOverlap
  (params (OtherActor :type Actor%20Object%20Reference)))

(event EventTick
  (params (DeltaSeconds :type Float%20%28single-precision%29)))

(fn ConstructionScript)