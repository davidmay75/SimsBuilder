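; BP_DefaultPawn is a camera pawn that exposes events for moving, zooming, orbiting and pitching the view.
; Movement input follows the actor's forward and right vectors, while zoom changes the spring arm's length.
; Orbit yaws the whole actor, and pitch rotates only the spring arm within clamped angles, both scaled by OrbitSpeed.
; A height event repositions the pawn's Z using a grid actor's offset and a new grid height.
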(event Custom|CameraOrbit
  (params (Magnitude :type Float%20%28single-precision%29))
  ;[1 1 1] Orbit and Pitch
  (Class|Actor|AddActorWorldRotation (Math|Rotator|MakeRotator 0.0 0.0 (* Magnitude (Variables|Default|GetOrbitSpeed)))))

(event Custom|MoveForwardBackward
  (params (Magnitude :type Float%20%28single-precision%29))
  ;[1 1 1] Forward
  (Pawn|Input|AddMovementInput (Transformation|GetActorForwardVector) Magnitude false))

(event Custom|CameraZoom
  (params (Magnitude :type Float%20%28single-precision%29))
  (bind _springarm (Variables|Default|GetSpringArm))
  ;[1 1 1] Zoom
  (Variables|/Script/Engine.SpringArmComponent|SetTargetArmLength _springarm (+ (* Magnitude (Variables|Default|GetZoomSpeed)) (Variables|/Script/Engine.SpringArmComponent|GetTargetArmLength _springarm))))

(event Custom|CameraHeight
  (params (Grid :type BP%20Grid%20Object%20Reference) (NewGridHeight :type Float%20%28single-precision%29))
  (bind _returnvalue (Transformation|GetActorLocation))
  ;[1 1 1] Camera Height
  (bind _output_get (Variables|Default|SetGridCameraDelta (- (.z (Transformation|GetActorLocation Grid)) (.z _returnvalue))))
  (Transformation|SetActorLocation (Math|Vector|MakeVector (.x _returnvalue) (.y _returnvalue) (+ _output_get NewGridHeight)) false false))

(event Custom|CameraPitch
  (params (Magnitude :type Float%20%28single-precision%29))
  (bind _springarm (Variables|Default|GetSpringArm))
  (bind _returnvalue (Transformation|GetWorldRotation _springarm))
  ;[1 1 1] Orbit and Pitch
  (Transformation|SetWorldRotation _springarm (Math|Rotator|MakeRotator (.roll _returnvalue) (Math|Float|ClampAngle (+ (* (Variables|Default|GetOrbitSpeed) Magnitude) (.pitch _returnvalue)) (Variables|Default|GetCameraMinClamp) (Variables|Default|GetCameraMaxClamp)) (.yaw _returnvalue)) false false))

(event Custom|MoveLeftRight
  (params (Magnitude :type Float%20%28single-precision%29))
  ;[1 1 1] Sideways
  (Pawn|Input|AddMovementInput (Transformation|GetActorRightVector) Magnitude false))

(event EventBeginPlay)

(fn ConstructionScript)